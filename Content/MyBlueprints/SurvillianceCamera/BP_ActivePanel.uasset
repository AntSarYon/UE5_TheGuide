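; BP_ActivePanel is a status panel for the surveillance camera system, showing a camera's label and whether it is active.
; It starts deactivated on BeginPlay.
; CamActivated and CamDeactivated swap the Panel material and set the state text to ON or OFF.
; AssignCameraNumber builds the "Cam-" label from the number passed to it.
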(event Custom|CamActivated
  ;[0.3854 0.1076 0] Evento | CamaraActivada
  (Rendering|Material|SetMaterial (Variables|Default|GetPanel) 0 (Variables|Default|GetMat_Active))
  (Rendering|Components|TextRender|SetText (Variables|Default|GetStateText) (Utilities|Text|MakeLiteralText "ON")))

(event Custom|CamDeactivated
  ;[0.3854 0.1076 0] Evento | Camara Desactivada
  (Rendering|Material|SetMaterial (Variables|Default|GetPanel) 0 (Variables|Default|GetMat_Deactive))
  (Rendering|Components|TextRender|SetText (Variables|Default|GetStateText) (Utilities|Text|MakeLiteralText "OFF")))

(event EventBeginPlay
  ;[1 1 1] Empezamos con el Panel Desactivado
  (CallFunction|CamDeactivated))

(event Collision|EventActorBeginOverlap
  (params (OtherActor :type Actor%20Object%20Reference)))

(event EventTick
  (params (DeltaSeconds :type Float%20%28single-precision%29)))

(fn ConstructionScript)

(fn AssignCameraNumber
  (params (CamNumber :type Integer))
  (Rendering|Components|TextRender|SetText (Variables|Default|GetCamNumberText) (Utilities|Text|ToText(String) (Utilities|String|Append "Cam-" (Utilities|String|ToString(Integer) CamNumber)))))