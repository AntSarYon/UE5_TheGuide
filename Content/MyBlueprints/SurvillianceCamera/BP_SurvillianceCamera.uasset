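; BP_SurvillianceCamera is a surveillance camera unit with a physics plug that the player connects to a BP_Socket to activate it.
; Tick toggles an interaction widget prompting grab or plug-in, based on the player's aim and socket proximity tracked by overlaps.
; Externally triggered connect and disconnect events toggle plug physics (snapping it to the socket on connect), play sounds, update the state panel and notify the player's camera button.
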(event OnComponentBeginOverlap(SocketDetectionArea)
  (params (OverlappedComponent :type Primitive%20Component%20Object%20Reference) (OtherActor :type Actor%20Object%20Reference) (OtherComp :type Primitive%20Component%20Object%20Reference) (OtherBodyIndex :type Integer) (bFromSweep :type Boolean) (SweepResult :type Hit%20Result%20Structure%20%28by%20ref%29))
  ;[1 0.2188 0.2188] Si un Socket esta en las proximidades, activamos el Flag de Socket cercano, y lo asignamos a la Variable de Socket
  (bind _asbp_socket (Utilities|Casting|CastToBP_Socket OtherActor))
  (Variables|Default|SetSocketNear true)
  (Variables|Default|SetAssignedSocket _asbp_socket))

(event OnComponentEndOverlap(SocketDetectionArea)
  (params (OverlappedComponent :type Primitive%20Component%20Object%20Reference) (OtherActor :type Actor%20Object%20Reference) (OtherComp :type Primitive%20Component%20Object%20Reference) (OtherBodyIndex :type Integer))
  ;[1 0.2291 0.239] Si un Socket sale del Trigger de Detección, desactivamos el Flag y quitamos su referencia de Socket asociado
  (Utilities|Casting|CastToBP_Socket OtherActor)
  (Variables|Default|SetSocketNear false)
  (Variables|Default|SetAssignedSocket 0))

(event Custom|PlugConected
  (bind _assignedsocket (Variables|Default|GetAssignedSocket))
  (bind _plugarea (Variables|/Game/MyBlueprints/SurvillianceCamera/BP_Socket.BP_Socket_C|GetPlugArea _assignedsocket))
  ;[1 0.0169 0] EVENTO: Enchufe Conectado
  ;;[1 1 1] Desactivamos las Fisicas del Enchufe
  (Physics|SetSimulatePhysics (Variables|Default|GetPlug_Mesh) false)
  ;;[1 1 1] Colocamos el Enchufe utilizando la ubicacion y rotación del Area de conexión del Socket como referencia
  (Transformation|SetWorldLocationAndRotation (Variables|Default|GetPlug_Mesh) (Transformation|GetWorldLocation _plugarea) (Transformation|GetWorldRotation _plugarea) true false)
  ;;[1 1 1] Reproducimos sonido de Conexión
  (Audio|PlaySoundatLocation "/Game/MySounds/Pluggin/PluggingInt_Cue.PluggingInt_Cue" (Transformation|GetWorldLocation (Variables|Default|GetPlug_Mesh)) "0, 0, 0" 1.0 1.0 0.0 0 0 0 0)
  ;;[1 1 1] Activamos Flag de CONECTADO
  (Variables|Default|SetIsConnected true)
  ;;[1 1 1] Invocamos el Evento de Activación del Panel
  (Default|CamActivated (Variables|Default|GetEstatePanel))
  ;;[1 1 1] Le decimos al Player que Active el boton asociado con esta camara
  (Default|EnableCameraButton (Variables|Default|GetPlayerReference) self))

(event Custom|PlugDesconnect
  ;[1 0.0169 0] EVENTO: Enchufe Desconectado
  ;;[1 1 1] Activamos las Fisicas del Enchufe
  (Physics|SetSimulatePhysics (Variables|Default|GetPlug_Mesh) true)
  ;;[1 1 1] Reproducimos sonido de Desconexión
  (Audio|PlaySoundatLocation "/Game/MySounds/Pluggin/PluggingOut_Cue.PluggingOut_Cue" (Transformation|GetWorldLocation (Variables|Default|GetPlug_Mesh)) "0, 0, 0" 1.0 1.0 0.0 0 0 0 0)
  ;;[1 1 1] Desactivamos Flag de CONECTADO
  (Variables|Default|SetIsConnected false)
  ;;[1 1 1] Invocamos le Evento de Desactivación del Panel
  (Default|CamDeactivated (Variables|Default|GetEstatePanel))
  ;;[1 1 1] Le decimos al Player que Desactive el boton asociado con esta camara
  (Default|EnableCameraButton (Variables|Default|GetPlayerReference) self))

(event EventBeginPlay
  ;[1 1 1] Obtenemos referencia al Jugador
  (CallFunction|GetPlayerReference)
  ;[1 1 1] Obtenemos referencia a Widget de Interaccion
  (CallFunction|GetWidgetReference)
  ;[1 1 1] Asignamos el Texto que tendrá el Widget
  (CallFunction|UpdateInteractionText)
  ;[1 1 1] Asignamos el Numero de la Camara al Panel
  (Default|AssignCameraNumber (Variables|Default|GetEstatePanel) (Variables|Default|GetCamNumber)))

(event Collision|EventActorBeginOverlap
  (params (OtherActor :type Actor%20Object%20Reference)))

(event EventTick
  (params (DeltaSeconds :type Float%20%28single-precision%29))
  ;[1 0.1751 0.1453] Revisamos si el Player esta apuntando hacia el Enchufe mientras se encuentra libre
  (bind _returnvalue (CallFunction|CheckIsPlayerViewingPlug))
  (if _returnvalue
    ;[1 0.07239 0.06244] Actualizamos el Texto de interacción del Widget
    (Variables|Default|SetInteractionText "Agarrar")
    (CallFunction|UpdateInteractionText)
    ;[1 0.0148 0] Activaremos la visibilidad del Wisget
    (Rendering|SetVisibility (Variables|Default|GetWidget) true false :!label _label)
    (else
      ;[1 0.0169 0] En caso de que NO, desactivaremos la visibilidad del Widget
      (Rendering|SetVisibility (Variables|Default|GetWidget) false false)
      ;[1 0.1245 0.1145] Revisamos si el Enchufe esta conectado
      (if (not (Variables|Default|GetIsConnected))
        ;[1 0.1245 0.1145] Revisamos si hay un Socket cercano...
        (if (Variables|Default|GetSocketNear)
          ;[1 0.07239 0.06244] Actualizamos el Texto de interacción del Widget
          (Variables|Default|SetInteractionText "Enchufar")
          (CallFunction|UpdateInteractionText)
          (goto _label)
          (else
            ;[1 0.0169 0] Desactivaremos la visibilidad del HUD
            (Rendering|SetVisibility (Variables|Default|GetWidget) false false)))))))

(fn ConstructionScript)

(fn GetPlayerReference
  (bind _asbp_tgplayer_character (Utilities|Casting|CastToBP_TGPlayerCharacter (Pawn|GetControlledPawn (Game|GetPlayerController 0))))
  (Variables|Default|SetPlayerReference _asbp_tgplayer_character))

(fn GetAssignedCamera
  (return (Variables|Default|GetAssignedCamera)))

(fn GetWidgetReference
  (bind _asw_interaction_prompt (Utilities|Casting|CastToW_InteractionPrompt (UserInterface|GetWidget (Variables|Default|GetWidget))))
  (Variables|Default|SetW_InteractPrompt _asw_interaction_prompt))

(fn UpdateInteractionText
  (Rendering|Components|TextRender|SetText (Variables|/Game/MyUI/W_InteractionPrompt.W_InteractionPrompt_C|GetTxtInteraction (Variables|Default|GetW_InteractPrompt)) (Variables|Default|GetInteractionText)))

(fn GetIsConnected
  (return (Variables|Default|GetIsConnected)))

(fn GetSocketNear
  (return (Variables|Default|GetSocketNear)))

(fn CheckIsPlayerViewingPlug
  (bind _playerreference (Variables|Default|GetPlayerReference))
  (return (and (== (Default|GetTargetMesh _playerreference) (Variables|Default|GetPlug_Mesh)) (not (Default|GetIsGrabbing _playerreference)))))

(fn GetCameraNumber
  (return (Variables|Default|GetCamNumber)))