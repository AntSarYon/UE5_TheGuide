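; BP_InteractableObject is an interactable world object that shows an interaction prompt widget to the player.
; On BeginPlay it caches the BP_TGPlayerCharacter and its W_InteractionPrompt widget, then sets the prompt text from InteractionText.
; Every Tick it shows the widget only while the player's target mesh is this object's StaticMesh and the player is not grabbing.
; TriggerInteraction calls CameraFadeIn on the player.
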(event Custom|TriggerInteraction
  (Default|CameraFadein (Variables|Default|GetPlayerReference)))

(event EventBeginPlay
  ;[1 1 1] Obtenemos referencia al Character del Jugador
  (CallFunction|GetPlayerReference)
  ;[1 1 1] Obtenemos referencia al Widget de Interacción utilizado
  (CallFunction|GetIPWidgetReference)
  ;[1 1 1] Asignamos el Texto que tendrá el TXT de Interaccion
  (CallFunction|SetIPWInteractionText))

(event EventTick
  (params (DeltaSeconds :type Float%20%28single-precision%29))
  ;[1 1 1] Manejamos la Visibilidad del HUD
  (CallFunction|ManageHUDVisibility))

(fn ConstructionScript)

(fn GetPlayerReference
  (bind _asbp_tgplayer_character (Utilities|Casting|CastToBP_TGPlayerCharacter (Pawn|GetControlledPawn (Game|GetPlayerController 0))))
  (Variables|Default|SetPlayerReference _asbp_tgplayer_character))

(fn GetIPWidgetReference
  (bind _asw_interaction_prompt (Utilities|Casting|CastToW_InteractionPrompt (UserInterface|GetWidget (Variables|Default|GetWidget))))
  (Variables|Default|SetW_InteractPrompt _asw_interaction_prompt))

(fn SetIPWInteractionText
  (Rendering|Components|TextRender|SetText (Variables|/Game/MyUI/W_InteractionPrompt.W_InteractionPrompt_C|GetTxtInteraction (Variables|Default|GetW_InteractPrompt)) (Variables|Default|GetInteractionText)))

(fn ManageHUDVisibility
  (bind _playerreference (Variables|Default|GetPlayerReference))
  ;[1 0.1751 0.1453] Revisamos si el TargetMesh del Personaje somos nosotros, y si está, o no, agarrando algún objeto
  (if (and (== (Default|GetTargetMesh _playerreference) (Variables|Default|GetStaticMesh)) (not (Default|GetIsGrabbing _playerreference)))
    ;[1 0.0148 0] Activaremos la visibilidad del HUD
    (Rendering|SetVisibility (Variables|Default|GetWidget) true false)
    (else
      ;[1 0.0169 0] Desactivaremos la visibilidad del HUD
      (Rendering|SetVisibility (Variables|Default|GetWidget) false false))))